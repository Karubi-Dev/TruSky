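; Player-controlled airplane that flies by applying forces and torques to its physics body, Driver.
; Roll, MoveRight and MoveForward axes apply roll, yaw and pitch torques scaled by Aircontroll.
; A looping ThrottleInput timer steps the clamped throttle while up or down is held, printing it on screen.
; Each Tick counters spin, adds constant downward acceleration, and blends velocity toward the nose direction at a throttle-based speed.
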(event `self.ReceiveTick`
  (params (DeltaSeconds :type "Float (single-precision)"))
  (bind _driver (`self.Driver`))
  (`PrimitiveComponent.AddTorqueInDegrees` _driver (/ (`KismetMathLibrary.NegateVector` (`PrimitiveComponent.GetPhysicsAngularVelocityInDegrees` (`self.Driver`) "None")) 0.5) "None" true)
  (`PrimitiveComponent.AddForce` _driver (0.0 0.0 -1500.0) "None" true)
  (`self.CalculateSpeed`))

(event `InputAxis|Roll`
  (params (AxisValue :type "Float (single-precision)"))
  (`PrimitiveComponent.AddTorqueInDegrees` (`self.Driver`) (`KismetMathLibrary.VLerp` (* (`SceneComponent.GetForwardVector` (`self.Driver`)) (* AxisValue (`self.Aircontroll`)))) "None" true))

(event `InputAction|ThrottleUp`
  (params (Key :type "Key Structure"))
  (:`Pressed`
    (set `self.ThrottleUp` true))
  (:`Released`
    (set `self.ThrottleUp` false)))

(event `InputAction|ThrottleDown`
  (params (Key :type "Key Structure"))
  (:`Pressed`
    (set `self.ThrottleDown` true))
  (:`Released`
    (set `self.ThrottleDown` false)))

(event `InputAxis|MoveRight`
  (params (AxisValue :type "Float (single-precision)"))
  (`PrimitiveComponent.AddTorqueInDegrees` (`self.Driver`) (`KismetMathLibrary.VLerp` (* (`SceneComponent.GetUpVector` (`self.Driver`)) (* AxisValue (`self.Aircontroll`)))) "None" true))

(event `self.ReceiveBeginPlay`
  (`KismetSystemLibrary.K2_SetTimer` null "ThrottleInput" 0.05 true))

(event `InputAxis|MoveForward`
  (params (AxisValue :type "Float (single-precision)"))
  (`PrimitiveComponent.AddTorqueInDegrees` (`self.Driver`) (`KismetMathLibrary.VLerp` (* (`SceneComponent.GetRightVector` (`self.Driver`)) (* AxisValue (`self.Aircontroll`)))) "None" true))

(fn `CalculateSpeed`
  (bind _driver (`self.Driver`))
  (bind _returnvalue (`PrimitiveComponent.GetPhysicsLinearVelocity` _driver "None"))
  (`PrimitiveComponent.SetPhysicsLinearVelocity` (`self.Driver`) (`KismetMathLibrary.VLerp` _returnvalue (* (`SceneComponent.GetForwardVector` _driver) (`KismetMathLibrary.FClamp` (* (`self.ThrottleAmount`) 250.0) 0.0 25000.0)) 0.01) false "None"))

(fn `ThrottleInput`
  (bind _throttleamount (`self.ThrottleAmount`))
  (if (`self.ThrottleUp`)
    (bind _result (`/Engine/EditorBlueprintResources/StandardMacros.IncrementInt` _throttleamount)
      (:`  `
        (bind _output_get (set `self.ThrottleAmount` (`KismetMathLibrary.Clamp` _result 1 100)))
        (`KismetSystemLibrary.PrintString` (`KismetStringLibrary.Conv_IntToString` _output_get))))
    (elif (`self.ThrottleDown`)
      (bind _result_2 (`/Engine/EditorBlueprintResources/StandardMacros.DecrementInt` _throttleamount)
        (:`  `
          (bind _output_get_2 (set `self.ThrottleAmount` (`KismetMathLibrary.Clamp` _result_2 1 100)))
          (`KismetSystemLibrary.PrintString` (`KismetStringLibrary.Conv_IntToString` _output_get_2)))))))

(fn `UserConstructionScript`)